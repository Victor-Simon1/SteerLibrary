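; BP_MyNode is a clickable node actor that links to successor nodes in Suiv and can be handed to a MyVehicle.
; On BeginPlay it prints debug text and line-traces against Pawns from each successor to itself with persistent black debug lines, leaving the hit result unused.
; When clicked, it prints its name and passes itself to AddNode on the first MyVehicle found in the level.
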(event EventBeginPlay
  (Development|PrintString "Begin")
  (for _array_element (Variables|Default|Getsuiv)
    (Development|PrintString (Utilities|GetDisplayName _array_element))
    (bind _outhit (Collision|LineTraceForObjects (Transformation|GetActorLocation _array_element) (Transformation|GetActorLocation self) (Utilities|Array|MakeArray "ObjectTypeQuery3") false 0 "Persistent" true "(R=0.000000,G=0.000000,B=0.000000,A=1.000000)"))
    (Development|PrintString "Hello")))

(event Collision|EventActorBeginOverlap
  (params (OtherActor :type Actor%20Object%20Reference)))

(event EventTick
  (params (DeltaSeconds :type Float%20%28single-precision%29)))

(event MouseInput|EventActorOnClicked
  (params (ButtonPressed :type Key%20Structure :default "None"))
  (Development|PrintString (Utilities|GetDisplayName self))
  (bind _outactors (Actor|GetAllActorsOfClass "/Game/Blueprints/MyVehicle.MyVehicle_C"))
  (bind _asmy_vehicle (Utilities|Casting|CastToMyVehicle (Utilities|Array|Get(acopy) _outactors)))
  (Default|AddNode _asmy_vehicle self))

(fn ConstructionScript)