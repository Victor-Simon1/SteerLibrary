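; MyVehicle is a vehicle actor that moves along node paths found by A* search.
; In the Minimal_Default level, once the game instance's pathfinding flag is set, Tick drives one-point, several-point or circuit movement by Mode; elsewhere it runs MoveTP1.
; AddNode collects selected target nodes, and PathFinding, in Mode 0 only, stores and prints the A* path from the first node to the first selection.
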(event Custom|AddNode
  (params (Actor :type BP%20My%20Node%20Object%20Reference))
  (Utilities|Array|Add (Variables|Default|GetseletectedNode) Actor))

(event Custom|PathFinding
  (if (== (Variables|Default|Getmode) 0)
    (bind _returnvalue (Class|Vehicle|AStar (Variables|Default|GetFirstNode) (Utilities|Array|Get(acopy) (Variables|Default|GetseletectedNode))))
    (bind _output_get (Variables|Default|SetpathToAccomplish _returnvalue))
    (Variables|Default|SetfinishSearch true)
    (for _array_element _output_get
      (Development|PrintString (Utilities|GetDisplayName _array_element) true true "(R=0.000000,G=0.660000,B=1.000000,A=1.000000)" 1.8e+02))))

(event EventBeginPlay)

(event Collision|EventActorBeginOverlap
  (params (OtherActor :type Actor%20Object%20Reference)))

(event EventTick
  (params (DeltaSeconds :type Float%20%28single-precision%29))
  (bind _returnvalue (Game|GetCurrentLevelName true))
  (if (Utilities|Enum|Equal(Enum) "Minimal_Default" _returnvalue)
    (bind _asbp_my_game_instance (Utilities|Casting|CastToBP_MyGameInstance (Game|GetGameInstance)))
    (if (Variables|/Game/Blueprints/BP_MyGameInstance.BP_MyGameInstance_C|GetPressPathFinding _asbp_my_game_instance)
      (if (== (Variables|Default|Getmode) 0)
        (Class|Vehicle|OnePoint DeltaSeconds)
        (elif (== (Variables|Default|Getmode) 1)
          (Class|Vehicle|SeveralPoint DeltaSeconds)
          (else
            (Class|Vehicle|Circuit2 DeltaSeconds)))))
    (else
      (Class|Vehicle|MoveTP1 DeltaSeconds))))

(fn ConstructionScript)