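; Player Blueprint that drives a single MyVehicle through debug-style input actions.
; On BeginPlay it caches the first MyVehicle actor found in the level.
; The BeginPathfinding input calls NewFunction0 on BP_MyGameInstance, then triggers the vehicle's PathFinding.
; The ChangeModeTP2 input switches the vehicle's mode and prints the new mode to screen.
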(event EventBeginPlay
  (bind _outactors (Actor|GetAllActorsOfClass "/Game/Blueprints/MyVehicle.MyVehicle_C"))
  (Variables|Default|SetVehicle (Utilities|Array|Get(acopy) _outactors)))

(event Collision|EventActorBeginOverlap
  (params (OtherActor :type Actor%20Object%20Reference)))

(event EventTick
  (params (DeltaSeconds :type Float%20%28single-precision%29)))

(event Input|ActionEvents|InputActionBeginPathfinding
  (params (Key :type Key%20Structure :default "None"))
  (:Pressed
    (bind _asbp_my_game_instance (Utilities|Casting|CastToBP_MyGameInstance (Game|GetGameInstance)))
    (Default|NewFunction0 _asbp_my_game_instance)
    (Development|PrintString "SearchPath")
    (Default|PathFinding (Variables|Default|GetVehicle))))

(event Input|ActionEvents|InputActionChangeModeTP2
  (params (Key :type Key%20Structure :default "None"))
  (bind _vehicle (Variables|Default|GetVehicle))
  (:Pressed
    (Class|Vehicle|ChangeMode _vehicle)
    (Development|PrintString (Utilities|String|ToString(Integer) (Variables|/Script/Steer.Vehicle|Getmode _vehicle)))))

(fn ConstructionScript)